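; Card deck actor that builds a visible stack of skeletal-mesh cards, with events to reload it or remove a card.
; On BeginPlay or reload, a looping timer adds cards one by one at stepped heights until NumberOfCards is reached.
; Each new card sets rise and fall flags on its ABP_SingleCard anim instance.
; Removal destroys the indexed component but leaves its array entry, as the RemoveIndex node is unconnected.
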(event `ReloadCards`
  (bind _cardmesharray (`self.CardMeshArray`))
  (for _array_element _cardmesharray
    (if (`KismetSystemLibrary.IsValid` _array_element)
      (`ActorComponent.K2_DestroyComponent` _array_element)))
  (`KismetArrayLibrary.Array_Clear` _cardmesharray)
  (bind _returnvalue (`KismetSystemLibrary.K2_SetTimerDelegate` (delegate `SpawnCards`) 0.05 true :!label _label)))

(event `SpawnCards`
  (bind _returnvalue (`KismetArrayLibrary.Array_Length` (`self.CardMeshArray`)))
  (bind _returnvalue_2 (`AddComponent|NODE_AddSkeletalMeshComponent-0` :`RelativeTransform` (`KismetMathLibrary.MakeTransform` (`KismetMathLibrary.MakeVector` 0.0 0.0 (* (+ _returnvalue -1) 0.17)))))
  (`KismetArrayLibrary.Array_Add` (`self.CardMeshArray`) _returnvalue_2)
  (bind _asabp_single_card (cast `/Game/FBXTest/SingleCardTest/ABP_SingleCard` (`SkeletalMeshComponent.GetAnimInstance` _returnvalue_2)))
  (set `/Game/FBXTest/SingleCardTest/ABP_SingleCard.ToRise` true _asabp_single_card)
  (set `/Game/FBXTest/SingleCardTest/ABP_SingleCard.ToFall` true _asabp_single_card)
  (if (== _returnvalue (`self.NumberOfCards`))
    (`KismetSystemLibrary.K2_ClearAndInvalidateTimerHandle` (stale `ReloadCards` _returnvalue))))

(event `self.ReceiveBeginPlay`
  (goto _label))

(event `self.RemoveCardFromDeck`
  (params (CardIndex :type Integer))
  (`ActorComponent.K2_DestroyComponent` (`|GetArrayItem` (`self.CardMeshArray`) CardIndex)))

(fn `UserConstructionScript`)